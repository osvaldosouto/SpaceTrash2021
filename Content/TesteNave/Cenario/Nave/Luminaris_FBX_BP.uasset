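; Luminaris ship Blueprint in the TesteNave area that moves itself from player axis input.
; MoveRight offsets the actor along its forward vector and MoveForward along its right vector, so the axes are crossed relative to their names.
; Each input event sets the location directly by a fixed step scaled by axis value, with no delta-time scaling or collision sweep.
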(event Input|AxisEvents|InputAxisMoveForward
  (params (AxisValue :type Float%20%28single-precision%29))
  (Transformation|SetActorLocation (+ (* (Transformation|GetActorRightVector) (* AxisValue 2e+02)) (Transformation|GetActorLocation)) false false))

(event Input|AxisEvents|InputAxisMoveRight
  (params (AxisValue :type Float%20%28single-precision%29))
  (Transformation|SetActorLocation (+ (* (Transformation|GetActorForwardVector) (* AxisValue 2e+02)) (Transformation|GetActorLocation)) false false))

(fn ConstructionScript)